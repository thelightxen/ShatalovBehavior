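; BP_Radio is an interactable radio object that toggles on and off when used.
; Each OnAction event flips the On flag, then shows its point light and starts its audio from the beginning, or hides the light and stops the audio.
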(event `OnAction`
  (bind _pointlight (`self.PointLight`))
  (bind _output_get (set `self.On?` (not (`self.On?`))))
  (if _output_get
    (`SceneComponent.SetVisibility` _pointlight true false)
    (`AudioComponent.Play` (`self.Audio`) 0.0)
    (else
      (`SceneComponent.SetVisibility` _pointlight false false)
      (`AudioComponent.Stop` (`self.Audio`)))))

(fn `UserConstructionScript`)