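; BP_Sosed is an NPC actor driven by a nested behavior system, starting BehHouseWork on BeginPlay.
; When it hits a BP_Box while not already pushing, it launches BehPushActors under the most recent behavior.
; That child is created unready, given the box and impact point, then started with Ready.
; Tick prints the active behavior hierarchy on screen for debugging.
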(event `self.ReceiveBeginPlay`
  (`Behavior.RunBehavior` (`self.Behavior`) "/Game/Behavior/BehHouseWork.BehHouseWork_C" true))

(event `self.ReceiveTick`
  (params (DeltaSeconds :type "Float (single-precision)"))
  (bind _returnvalue (`Behavior.GetDebugHierarchi` (`self.Behavior`)))
  (`KismetSystemLibrary.PrintString` (`KismetStringLibrary.Concat_StrStr` "\"" (`KismetStringLibrary.JoinStringArray` _returnvalue "\" > \" ") "\"") true false (struct :`G` 1.0 :`A` 1.0) 0.0))

(event `self.ReceiveHit`
  (params (MyComp :type "PrimitiveComponent Object Reference") (Other :type "Actor Object Reference") (OtherComp :type "PrimitiveComponent Object Reference") (bSelfMoved :type Boolean) (HitLocation :type "Vector Structure") (HitNormal :type "Vector Structure") (NormalImpulse :type "Vector Structure") (Hit :type "HitResult Structure (by ref)"))
  ;[1 1 1] Check if actors on path
  (bind _asbp_box (cast `/Game/Objects/BP_Objects/BP_Box` Other))
  (if (not (`self.IsPushing?`))
    (bind _returnvalue (`Behavior.GetLastBehavior` (`self.Behavior`)))
    (bind _returnvalue_2 (`Behavior.RunBehavior` _returnvalue "/Game/Behavior/Idle/BehPushActors.BehPushActors_C" false))
    (bind _asbeh_push_actors (cast `/Game/Behavior/Idle/BehPushActors` _returnvalue_2 :!pure true))
    (set `/Game/Behavior/Idle/BehPushActors.ActorToPush` _asbp_box _asbeh_push_actors)
    (set `/Game/Behavior/Idle/BehPushActors.ImpactPoint` (`.ImpactPoint` (`GameplayStatics.BreakHitResult` Hit)) _asbeh_push_actors)
    (`Behavior.Ready` _asbeh_push_actors)))

(fn `UserConstructionScript`)