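; BP_BehaviorOwner is a Blueprint that runs a behavior through its Behavior object and shows that behavior's state on screen for debugging.
; After a short delay at BeginPlay, it starts BehMain through RunBehavior, flagged as ready.
; Every Tick it prints whether the behavior is interrupted, plus the debug hierarchy joined into a single green line.
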(event `self.ReceiveBeginPlay`
  (`KismetSystemLibrary.Delay` 0.2)
  (`Behavior.RunBehavior` (`self.Behavior`) "/Game/Tasks/BehMain.BehMain_C" true))

(event `self.ReceiveTick`
  (params (DeltaSeconds :type "Float (single-precision)"))
  (bind _behavior (`self.Behavior`))
  (`KismetSystemLibrary.PrintString` (`KismetStringLibrary.Concat_StrStr` "IsInterrupted: " (`KismetStringLibrary.Conv_BoolToString` (`Behavior.IsInterrupted` _behavior))) true false (struct :`G` 0.66 :`B` 1.0 :`A` 1.0) 0.0)
  (bind _returnvalue (`Behavior.GetDebugHierarchi` _behavior))
  (`KismetSystemLibrary.PrintString` (`KismetStringLibrary.JoinStringArray` _returnvalue " > ") true false (struct :`G` 1.0 :`A` 1.0) 0.0))

(fn `UserConstructionScript`)